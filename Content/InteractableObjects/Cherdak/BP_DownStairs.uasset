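; Interactable attic stairway that takes the player down once the "Чердак" (attic) quest is completed, and otherwise shows a dialogue line saying to finish here first.
; On success it deactivates the linked up-stairs object, fades the HUD out, moves the player to a teleport point and fades back in.
; It then runs the parent interaction and adds the "KuhnyaGaz" quest.
; Entering its trigger enables the interact button and custom-depth rendering on the mesh.
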(event `/Game/InteractableObjects/BP_Interact.Interact`
  (bind _teleportpoint (`self.TeleportPoint`))
  (bind _w_hud (`/Game/TopDownBP/Blueprints/TopDownGameMode.W_HUD` (cast `/Game/TopDownBP/Blueprints/TopDownGameMode` (`GameplayStatics.GetGameMode`) :!pure true)))
  (bind _fadescreen (`/Game/HUD/W_HUD.FadeScreen` _w_hud))
  (if (`/Game/QuestSystem/BPs/BPC_QuestManager.IsQuestCompleted?` (`/Game/TopDownBP/Blueprints/TopDownCharacter.BPC_QuestManager` (`self.MainCharRef`)) "Чердак")
    (set `/Game/InteractableObjects/Cherdak/BP_UpStairs.isActive?` false (`self.BP_UpStairs`))
    (`|PlayAnimation` _w_hud _fadescreen
      (:`Finished`
        (`self.K2_SetActorLocationAndRotation` (`GameplayStatics.GetPlayerCharacter` 0) (`self.K2_GetActorLocation` _teleportpoint) (`self.K2_GetActorRotation` _teleportpoint) false false)
        (`|PlayAnimation` _w_hud _fadescreen 0.0 1 "Reverse"
          (:`Finished`
            (`parent.Interact`)
            (`/Game/QuestSystem/BPs/BPC_QuestManager.AddQuest` (`/Game/TopDownBP/Blueprints/TopDownCharacter.BPC_QuestManager` (`self.MainCharRef`)) "KuhnyaGaz")))))
    (else
      (`/Game/HUD/Dialogue/W_DialogueWindow.OpenDialogueWidget` (`/Game/HUD/W_HUD.W_DialogueWindow` _w_hud) (`|MakeArray` "Сначала нужно закончить здесь." :!type "Text")))))

(fn `OnTriggerEnter`
  (`self.Set Interact Button Enabled`)
  (`PrimitiveComponent.SetRenderCustomDepth` (`self.StaticMesh`) true))

(fn `UserConstructionScript`
  (`parent.UserConstructionScript`))