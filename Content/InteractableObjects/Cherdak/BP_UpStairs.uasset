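; BP_UpStairs is an interactable stairs object that teleports the player character to a TeleportPoint behind a screen fade.
; Interact plays the HUD's FadeScreen animation, teleports to the point's location and rotation, reverses the fade, then calls the parent Interact once that finishes.
; OnTriggerEnter, when the object is active, enables the interact button and turns on custom depth rendering for the mesh.
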(event `/Game/InteractableObjects/BP_Interact.Interact`
  (bind _teleportpoint (`self.TeleportPoint`))
  (bind _w_hud (`/Game/TopDownBP/Blueprints/TopDownGameMode.W_HUD` (cast `/Game/TopDownBP/Blueprints/TopDownGameMode` (`GameplayStatics.GetGameMode`) :!pure true)))
  (bind _fadescreen (`/Game/HUD/W_HUD.FadeScreen` _w_hud))
  (`|PlayAnimation` _w_hud _fadescreen
    (:`Finished`
      (`self.K2_TeleportTo` (`GameplayStatics.GetPlayerCharacter` 0) (`self.K2_GetActorLocation` _teleportpoint) (`self.K2_GetActorRotation` _teleportpoint))
      (`|PlayAnimation` _w_hud _fadescreen 0.0 1 "Reverse"
        (:`Finished`
          (`parent.Interact`))))))

(fn `OnTriggerEnter`
  (if (`self.isActive?`)
    (`self.Set Interact Button Enabled`)
    (`PrimitiveComponent.SetRenderCustomDepth` (`self.StaticMesh`) true)))

(fn `UserConstructionScript`
  (`parent.UserConstructionScript`))