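; Interactable electrical switchboard that opens the HUD switchboard widget once the "Чердак" (attic) and "Запах из кухни" (kitchen gas smell) quests are completed.
; Until then, interacting shows a dialogue naming the unfinished prerequisite.
; On opening, it hands the player's quest manager to the widget and refreshes its buttons.
; Trigger entry enables the interact button and custom-depth rendering; parent overlap handling is skipped during the "Установить УЗО" (install RCD) subgoal.
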(event `self.ReceiveActorBeginOverlap`
  (params (OtherActor :type "Actor Object Reference"))
  (if (not (`KismetTextLibrary.EqualEqual_TextText` (`.SubGoalName_5_866E577649C18B9CAFC491966E332E8E` (break `/Game/QuestSystem/Data/S_SubGoal` (`/Game/QuestSystem/BPs/BPC_QuestManager.CurrentSubGoal` (`/Game/TopDownBP/Blueprints/TopDownCharacter.BPC_QuestManager` (`self.MainCharRef`))))) "Установить УЗО"))
    (`parent.ReceiveActorBeginOverlap` OtherActor)))

(event `/Game/InteractableObjects/BP_Interact.Interact`
  (bind _bpc_questmanager (`/Game/TopDownBP/Blueprints/TopDownCharacter.BPC_QuestManager` (`self.MainCharRef`)))
  (bind _w_hud (`/Game/TopDownBP/Blueprints/TopDownGameMode.W_HUD` (cast `/Game/TopDownBP/Blueprints/TopDownGameMode` (`GameplayStatics.GetGameMode`) :!pure true)))
  (bind _w_dialoguewindow (`/Game/HUD/W_HUD.W_DialogueWindow` _w_hud))
  (bind _w_switchboard (`/Game/HUD/W_HUD.W_SwitchBoard` _w_hud))
  (if (`/Game/QuestSystem/BPs/BPC_QuestManager.IsQuestCompleted?` _bpc_questmanager "Чердак")
    (if (`/Game/QuestSystem/BPs/BPC_QuestManager.IsQuestCompleted?` _bpc_questmanager "Запах из кухни")
      (`Widget.SetVisibility` _w_switchboard "Visible")
      (set `/Game/InteractableObjects/Widgets/W_SwitchBoard.QuestManager` _bpc_questmanager _w_switchboard)
      (`/Game/InteractableObjects/Widgets/W_SwitchBoard.UpdateButtons` _w_switchboard)
      (else
        (`/Game/HUD/Dialogue/W_DialogueWindow.OpenDialogueWidget` _w_dialoguewindow (`|MakeArray` "Сначала нужно разобраться с запахом газа на кухне." "Свет сейчас включать нельзя. Газ может взорваться!" :!type "Text"))))
    (else
      (`/Game/HUD/Dialogue/W_DialogueWindow.OpenDialogueWidget` _w_dialoguewindow (`|MakeArray` "Сначала нужно проверить чердак." :!type "Text")))))

(fn `OnTriggerEnter`
  (`self.Set Interact Button Enabled`)
  (`PrimitiveComponent.SetRenderCustomDepth` (`self.StaticMesh`) true))

(fn `UserConstructionScript`
  (`parent.UserConstructionScript`))