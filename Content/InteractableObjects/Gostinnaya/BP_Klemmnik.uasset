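; BP_Klemmnik is an interactable object that plays a UI animation sequence when the player interacts with it.
; Interact disables the Box collision, player input and virtual joystick, then shows the WKlemmnik widget from the TopDownGameMode HUD and plays its animation.
; When the animation finishes, it removes the widget, restores input and joystick, and only then calls the parent Interact, while collision stays off.
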(event `/Game/InteractableObjects/BP_Interact.Interact`
  (bind _returnvalue (`GameplayStatics.GetPlayerController` 0))
  (bind _returnvalue_2 (`GameplayStatics.GetPlayerController` 0))
  (bind _w_klemmnik (`/Game/HUD/W_HUD.W_Klemmnik` (`/Game/TopDownBP/Blueprints/TopDownGameMode.W_HUD` (cast `/Game/TopDownBP/Blueprints/TopDownGameMode` (`GameplayStatics.GetGameMode`) :!pure true))))
  (`PrimitiveComponent.SetCollisionEnabled` (`self.Box`) "NoCollision")
  (`self.DisableInput` (`self.MainCharRef`) _returnvalue_2)
  (`PlayerController.SetVirtualJoystickVisibility` _returnvalue_2 false)
  (`Widget.SetVisibility` _w_klemmnik "Visible")
  (`|PlayAnimation` _w_klemmnik (`/Game/HUD/Klemmnik/W_Klemmnik.123` _w_klemmnik)
    (:`Finished`
      (`Widget.RemoveFromParent` _w_klemmnik)
      (`self.EnableInput` (`self.MainCharRef`) _returnvalue)
      (`PlayerController.SetVirtualJoystickVisibility` _returnvalue true)
      (`parent.Interact`))))

(fn `UserConstructionScript`
  (`parent.UserConstructionScript`))