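; BP_QuestItem is an interactable world object that completes a quest sub-goal when the player uses it.
; On Interact it checks the current sub-goal in the main character's BPCQuestManager, triggering Game Over through TopDownGameMode if that sub-goal needs a phone ring.
; Otherwise it passes its SubGoalText to the quest manager, disables the interact button and turns off the mesh's custom-depth rendering.
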(event `self.ReceiveActorBeginOverlap`
  (params (OtherActor :type "Actor Object Reference"))
  (`parent.ReceiveActorBeginOverlap` OtherActor))

(event `/Game/InteractableObjects/BP_Interact.Interact`
  (bind (_currentsubgoal_subgoalname _currentsubgoal_dialogueafteraddinggoal _currentsubgoal_show_ _currentsubgoal_complete_ _currentsubgoal_needphonering_) (break `/Game/QuestSystem/Data/S_SubGoal` (`/Game/QuestSystem/BPs/BPC_QuestManager.CurrentSubGoal` (`/Game/TopDownBP/Blueprints/TopDownCharacter.BPC_QuestManager` (`self.MainCharRef`)))))
  (if (not _currentsubgoal_needphonering_)
    (bind _astop_down_character (cast `/Game/TopDownBP/Blueprints/TopDownCharacter` (`GameplayStatics.GetPlayerCharacter` 0)))
    (`/Game/QuestSystem/BPs/BPC_QuestManager.CompleteSubGoal` (`/Game/TopDownBP/Blueprints/TopDownCharacter.BPC_QuestManager` _astop_down_character) (`self.SubGoalText`))
    (`self.Set Interact Button Disabled`)
    (`PrimitiveComponent.SetRenderCustomDepth` (`self.StaticMesh`) false)
    (else
      ;[1 1 1] Game Over
      (bind _astop_down_game_mode (cast `/Game/TopDownBP/Blueprints/TopDownGameMode` (`GameplayStatics.GetGameMode`)))
      (`/Game/TopDownBP/Blueprints/TopDownGameMode.GameOver` _astop_down_game_mode))))

(fn `GetSubGoalText`
  (returns (SubGoal :type Text))
  (return (`self.SubGoalText`)))

(fn `UserConstructionScript`
  (`parent.UserConstructionScript`))