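; Quest-gated interactable actor that lets the player use the HUD interact button when standing inside its trigger box.
; On TopDownCharacter overlap, it compares its SubGoalText with the quest manager's current subgoal name.
; A match enables the button through the GameMode's HUD widget, sets its text and target, and highlights the mesh via custom depth.
; Leaving resets all of these; GetSubGoalText is a stub returning an empty string.
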(event `self.Box.OnComponentBeginOverlap`
  (params (OverlappedComponent :type "PrimitiveComponent Object Reference") (OtherActor :type "Actor Object Reference") (OtherComp :type "PrimitiveComponent Object Reference") (OtherBodyIndex :type Integer) (bFromSweep :type Boolean) (SweepResult :type "HitResult Structure (by ref)"))
  (bind _astop_down_character (cast `/Game/TopDownBP/Blueprints/TopDownCharacter` OtherActor))
  (set `self.MainCharRef` _astop_down_character)
  (`self.OnTriggerEnter`))

(event `self.Box.OnComponentEndOverlap`
  (params (OverlappedComponent :type "PrimitiveComponent Object Reference") (OtherActor :type "Actor Object Reference") (OtherComp :type "PrimitiveComponent Object Reference") (OtherBodyIndex :type Integer))
  (cast `/Game/TopDownBP/Blueprints/TopDownCharacter` OtherActor)
  (`self.Set Interact Button Disabled`)
  (`PrimitiveComponent.SetRenderCustomDepth` (`self.StaticMesh`) false))

(fn `GetSubGoalText`
  (returns (SubGoal :type Text))
  (return ""))

(fn `OnTriggerEnter`
  (bind _currentsubgoal_subgoalname (break `/Game/QuestSystem/Data/S_SubGoal` (`/Game/QuestSystem/BPs/BPC_QuestManager.CurrentSubGoal` (`/Game/TopDownBP/Blueprints/TopDownCharacter.BPC_QuestManager` (`self.MainCharRef`)))))
  (if (`KismetTextLibrary.EqualEqual_TextText` (`self.SubGoalText`) _currentsubgoal_subgoalname)
    (`self.Set Interact Button Enabled`)
    (`PrimitiveComponent.SetRenderCustomDepth` (`self.StaticMesh`) true)))

(fn `Set Interact Button Disabled`
  (bind _astop_down_game_mode (cast `/Game/TopDownBP/Blueprints/TopDownGameMode` (`GameplayStatics.GetGameMode`)))
  (bind _w_hud (`/Game/TopDownBP/Blueprints/TopDownGameMode.W_HUD` _astop_down_game_mode))
  (`Widget.SetIsEnabled` (`/Game/HUD/W_HUD.B_Interact` _w_hud) false)
  (`TextBlock.SetText` (`/Game/HUD/W_HUD.InteractionText` _w_hud) "Взаимодействие")
  (set `/Game/HUD/W_HUD.InteractableObject` null _w_hud))

(fn `Set Interact Button Enabled`
  (bind _astop_down_game_mode (cast `/Game/TopDownBP/Blueprints/TopDownGameMode` (`GameplayStatics.GetGameMode`)))
  (bind _w_hud (`/Game/TopDownBP/Blueprints/TopDownGameMode.W_HUD` _astop_down_game_mode))
  (`Widget.SetIsEnabled` (`/Game/HUD/W_HUD.B_Interact` _w_hud) true)
  (`TextBlock.SetText` (`/Game/HUD/W_HUD.InteractionText` _w_hud) (`self.InteractionText`))
  (set `/Game/HUD/W_HUD.InteractableObject` self _w_hud))

(fn `UserConstructionScript`)